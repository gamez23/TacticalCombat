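; BP_Grid_Debug is a debug version of a grid actor that tests grid shape lookups in DT_GridShapeData.
; The construction script passes the grid settings to SpawnGrid, which stores the shape and loops over the table's rows but spawns no tiles.
; For each row, it converts the shape enum to a Name, retries the lookup with that key, and prints color-coded working, broken or missing-row messages.
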(fn `SpawnGrid`
  (params (CenterLocation :type "Vector Structure") (TileSize :type "Vector Structure") (TileCount :type "Vector2D Structure") (Shape :type "/Game/Blueprints/Core/Grid/GridShapes/E_GridShape Enum" :default "NewEnumerator0"))
  (bind _output_get (set `self.GridShape` Shape))
  (bind _outrownames (`DataTableFunctionLibrary.GetDataTableRowNames` "/Game/Blueprints/Core/Grid/GridShapes/DT_GridShapeData.DT_GridShapeData"))
  (for _array_element _outrownames
    (bind _returnvalue (`|GetDataTableRow` "/Game/Blueprints/Core/Grid/GridShapes/DT_GridShapeData.DT_GridShapeData" _array_element)
      (:`then`
        (bind _returnvalue_2 (`|GetEnumeratorNameAsString` _output_get))
        (bind _returnvalue_3 (`KismetStringLibrary.Conv_NameToString` (`KismetStringLibrary.Conv_StringToName` _returnvalue_2)))
        (`KismetSystemLibrary.PrintString` (`KismetStringLibrary.Concat_StrStr` (`KismetStringLibrary.Conv_NameToString` (`|GetEnumeratorName` Shape)) "::" _returnvalue_2 "::" _returnvalue_3 "::") true true (struct :`R` 0.161992 :`G` 0.512903 :`B` 1.0 :`A` 1.0) 5.0)
        (bind _returnvalue_4 (`KismetStringLibrary.Conv_StringToName` _returnvalue_3))
        (`|GetDataTableRow` "/Game/Blueprints/Core/Grid/GridShapes/DT_GridShapeData.DT_GridShapeData" _returnvalue_4
          (:`then`
            (bind _returnvalue_5 (`KismetStringLibrary.Conv_NameToString` _returnvalue_4))
            (`KismetSystemLibrary.PrintString` (`KismetStringLibrary.Concat_StrStr` "WORKING::" _returnvalue_5) true true (struct :`R` 0.320916 :`G` 1.0 :`B` 0.448455 :`A` 1.0)))
          (:`RowNotFound`
            (`KismetSystemLibrary.PrintString` (`KismetStringLibrary.Concat_StrStr` "BROKEN::" _returnvalue_5) true true (struct :`R` 1.0 :`G` 0.81387 :`B` 0.481045 :`A` 1.0)))))
      (:`RowNotFound`
        (`KismetSystemLibrary.PrintString` (`KismetStringLibrary.Concat_StrStr` "ERROR:RowNotFound::" (`KismetStringLibrary.Conv_NameToString` _array_element)) true true (struct :`R` 1.0 :`G` 0.034294 :`A` 1.0) 5.0)))))

(fn `UserConstructionScript`
  (`self.SpawnGrid` (`self.GridCenterLocation`) (`self.GridTileSize`) (`self.GridTileCount`) (`self.GridShape`)))